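; Test Blueprint, named as a replicating component, that exercises a constructed BP_Container object and its nested Floater values.
; On BeginPlay, only the network authority constructs the container and stores it in Container.
; Every Tick, with no authority or validity check, it prints the Floater's Float1 and Float2, exposing what each network side holds.
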(event EventBeginPlay
  (Networking|SwitchHasAuthority
    (:Authority
      (bind _returnvalue (Game|ConstructObjectfromClass self "/Game/Tests/BP_Container.BP_Container_C"))
      (Variables|Default|SetContainer _returnvalue))))

(event EventTick
  (params (DeltaSeconds :type Float%20%28single-precision%29))
  (bind _container (Variables|Default|GetContainer))
  (bind _floater (Variables|/Game/Tests/BP_Container.BP_Container_C|GetFloater _container))
  (Development|PrintString (Utilities|String|Append (Utilities|String|ToString(Float) (Variables|/Game/Tests/BP_Floater.BP_Floater_C|GetFloat1 _floater)) "/" (Utilities|String|ToString(Float) (Variables|/Game/Tests/BP_Floater.BP_Floater_C|GetFloat2 _floater)))))