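; BP_TestActor3_Structs is a test actor that stores an object reference inside a struct and reads it back.
; On BeginPlay, only with authority, it constructs a BP_Floater and wraps it in a TestStruct held in the Struct variable.
; Every Tick, on any side, it casts the struct's first member to BP_Floater and prints its two float values in red, skipping when the cast fails.
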(event EventBeginPlay
  (Networking|SwitchHasAuthority
    (:Authority
      (bind _returnvalue (Game|ConstructObjectfromClass "/Game/Tests/BP_Floater.BP_Floater_C"))
      (Variables|Default|SetStruct (Utilities|Struct|MakeTestStruct _returnvalue)))))

(event EventTick
  (params (DeltaSeconds :type Float%20%28single-precision%29))
  (bind _asbp_floater (Utilities|Casting|CastToBP_Floater (Utilities|Struct|BreakTestStruct (Variables|Default|GetStruct))))
  (Development|PrintString (Utilities|String|Append (Utilities|String|ToString(Float) (Variables|/Game/Tests/BP_Floater.BP_Floater_C|GetFloat1 _asbp_floater)) "/" (Utilities|String|ToString(Float) (Variables|/Game/Tests/BP_Floater.BP_Floater_C|GetFloat2 _asbp_floater))) true true "(R=1.000000,G=0.000000,B=0.000000,A=1.000000)"))

(fn ConstructionScript)